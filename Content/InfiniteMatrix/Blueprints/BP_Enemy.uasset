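; BP_Enemy is an enemy actor that spins continuously around its yaw axis and reacts to overlaps on its mesh.
; Touching the player decrements their lives, then either marks them dead and shows the restart display at zero or destroys the enemy.
; A projectile hit spawns a particle burst, chosen by the player's powered state, destroys both actors and calls KillEnemy on the player.
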(event `self.ReceiveBeginPlay`)

(event `self.ReceiveTick`
  (params (DeltaSeconds :type "Float (single-precision)"))
  (`self.K2_AddActorLocalRotation` (`KismetMathLibrary.MakeRotator` 0.0 0.0 (* DeltaSeconds 30.0))))

(event `self.EnemyMesh.OnComponentBeginOverlap`
  (params (OverlappedComponent :type "PrimitiveComponent Object Reference") (OtherActor :type "Actor Object Reference") (OtherComp :type "PrimitiveComponent Object Reference") (OtherBodyIndex :type Integer) (bFromSweep :type Boolean) (SweepResult :type "HitResult Structure (by ref)"))
  (bind _asbp_player (cast `/Game/InfiniteMatrix/Blueprints/BP_Player` OtherActor)
    (:`then`
      (`/Game/InfiniteMatrix/Blueprints/BP_Player.DecrementLives` _asbp_player)
      (bind _returnvalue (== (`/Game/InfiniteMatrix/Blueprints/BP_Player.CurrentLives` _asbp_player) 0))
      (if _returnvalue
        (set `/Game/InfiniteMatrix/Blueprints/BP_Player.IsDead` _returnvalue _asbp_player)
        (`/Game/InfiniteMatrix/Blueprints/BP_Player.DisplayRestart` _asbp_player)
        (else
          (`self.K2_DestroyActor`))))
    (:`CastFailed`
      (bind _asbp_projectile (cast `/Game/InfiniteMatrix/Blueprints/BP_Projectile` OtherActor))
      (bind _asbp_player_2 (cast `/Game/InfiniteMatrix/Blueprints/BP_Player` (`GameplayStatics.GetPlayerPawn` 0)))
      (if (`/Game/InfiniteMatrix/Blueprints/BP_Player.IsPowered` _asbp_player_2)
        (bind _returnvalue_2 (`self.K2_GetActorLocation` _asbp_projectile))
        (`NiagaraFunctionLibrary.SpawnSystemAtLocation` "/Game/InfiniteMatrix/UI/ParticleBurst_PowerUp.ParticleBurst_PowerUp" _returnvalue_2)
        (else
          (`NiagaraFunctionLibrary.SpawnSystemAtLocation` "/Game/InfiniteMatrix/UI/ParticleBurst.ParticleBurst" _returnvalue_2)))
      (`self.K2_DestroyActor` _asbp_projectile)
      (`self.K2_DestroyActor`)
      (bind _asbp_player_3 (cast `/Game/InfiniteMatrix/Blueprints/BP_Player` (`GameplayStatics.GetPlayerPawn` 0)))
      (`/Game/InfiniteMatrix/Blueprints/BP_Player.KillEnemy` _asbp_player_3))))

(fn `UserConstructionScript`)